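; BP_Turtle is a moving turtle actor that tumbles end over end in 90-degree steps.
; Tick swings a vector derived from its bounds around the right axis to set location, while pitching the actor at Speed.
; Each finished step saves the new position and calls StepCompleted.
; BehaviourType then decides whether it continues straight, pauses after some steps, or pauses and reverses by negating Speed.
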(event `self.ReceiveBeginPlay`
  ;[1 1 1] Setup initial parameters
  (set `self.BodyExtent` (`.BoxExtent` (`self.GetActorBounds` false)))
  (set `self.LastVector` (`KismetMathLibrary.RotateAngleAxis` (* (`self.BodyExtent`) (1.0 0.0 -1.0)) (`KismetMathLibrary.SelectFloat` 180.0 90.0 (< (`self.Speed`) 0.0)) (`self.GetActorRightVector`)))
  (set `self.LastPosition` (`self.K2_GetActorLocation`)))

(event `self.ReceiveTick`
  (params (DeltaSeconds :type "Float (single-precision)"))
  (bind _returnvalue (< (`self.Speed`) 0.0))
  ;[1 1 1] turtle movement
  (if (`self.Moving`)
    (bind _output_get (set `self.Delta Seconds` DeltaSeconds))
    (bind _returnvalue_2 (* (`self.Speed`) _output_get))
    (bind _output_get_2 (set `self.LastDegree` (+ (stale _output_get_2) (`KismetMathLibrary.Abs` _returnvalue_2))))
    (bind _output_get_3 (set `self.LastVector` (`KismetMathLibrary.RotateAngleAxis` (stale _output_get_3) _returnvalue_2 (`self.GetActorRightVector`))))
    (`self.K2_SetActorLocation` (+ (`KismetMathLibrary.RotateAngleAxis` (* (`self.BodyExtent`) (`KismetMathLibrary.SelectVector` (-1.0 0.0 1.0) (-1.0 0.0 1.0) _returnvalue)) (`KismetMathLibrary.SelectFloat` 180.0 90.0 _returnvalue) (`self.GetActorRightVector`)) (`self.LastVector`) (`self.LastPosition`)))
    (`self.K2_AddActorLocalRotation` (`KismetMathLibrary.MakeRotator` 0.0 (* (`self.Speed`) -1.0 (`self.Delta Seconds`))))
    ;;[1 1 1] If step completed -> update position before next step
    (if (>= (`self.LastDegree`) 90.0)
      (set `self.LastPosition` (`self.K2_GetActorLocation`))
      (set `self.LastDegree` 0.0)
      (set `self.LastVector` (`self.GetNextStepVectorUpdate`))
      (set `self.Moving` false)
      (`self.StepCompleted`))))

(event `StepCompleted`
  (bind _returnvalue (>= (`self.StepsMade`) (`KismetMathLibrary.SelectInt` 1 4 (< (`self.Speed`) 0.0))))
  ;[1 1 1] Behaviours
  (switch `/Game/Blueprints/Game/Enum_BehaviorType` (`self.BehaviourType`)
    (:`NewEnumerator0`
      (set `self.Moving` true))
    (:`NewEnumerator1`
      (if _returnvalue
        (`KismetSystemLibrary.Delay` 1.0)
        (set `self.StepsMade` 0)
        (else
          (bind _output_get (set `self.StepsMade` (+ (stale _output_get) 1)))))
      (set `self.Moving` true))
    (:`NewEnumerator2`
      (if _returnvalue
        (set `self.StepsMade` 0)
        (`KismetSystemLibrary.Delay` 0.2)
        (bind _output_get_2 (set `self.Speed` (* (stale _output_get_2) -1.0)))
        (set `self.LastVector` (`self.GetNextStepVectorUpdate`))
        (else
          (bind _output_get_3 (set `self.StepsMade` (+ (stale _output_get_3) 1)))))
      (set `self.Moving` true))))

(fn `UserConstructionScript`)