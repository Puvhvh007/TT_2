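; BP_Nest is a spawner actor that releases turtles (BP_Turtle) at its own transform.
; Each ToggleNest call spawns a turtle only if the last one is no longer valid or is at least SafeDistance away from the nest.
; SpawnTurtle passes the nest's Behavior setting to the new turtle's BehaviourType and stores it as LastTurtle for the next check.
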(event `ToggleNest`
  (bind _lastturtle (`self.LastTurtle`))
  ;[1 1 1] Спавним след. черепаху, но только если старая черепаха далеко
  (`/Engine/EditorBlueprintResources/StandardMacros.IsValid` _lastturtle
    (:`Is Valid`
      (if (>= (`KismetMathLibrary.VSize` (- (`self.K2_GetActorLocation`) (`self.K2_GetActorLocation` _lastturtle))) (`self.SafeDistance`))
        (`self.SpawnTurtle` :!label _label)))
    (:`Is Not Valid`
      (goto _label))))

(fn `SpawnTurtle`
  ;[1 1 1] Spawn turtle and gift it with purpose
  (bind _returnvalue (`|SpawnActorFromClass` "/Game/Blueprints/Game/BP_Turtle.BP_Turtle_C" (`self.GetTransform`) "Undefined" "OverrideRootScale" null null))
  (set `/Game/Blueprints/Game/BP_Turtle.BehaviourType` (`self.Behavior`) _returnvalue)
  (set `self.LastTurtle` _returnvalue))

(fn `UserConstructionScript`)